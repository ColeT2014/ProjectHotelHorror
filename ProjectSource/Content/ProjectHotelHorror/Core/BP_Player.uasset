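; First-person player character for a hotel horror game, handling movement, walk/run, look and a reticle widget.
; While moving, a looping timer traces downward for surface-based carpet or wood footsteps, and Tick plays speed-based head-bob camera shakes.
; Interact line-traces from the camera to open hotel room doors.
; Amnesia-style drag interaction forwards mouse input and damps look while interacting, but its trace and release logic are disconnected.
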(event `InputAction|Run`
  (params (Key :type "Key Structure"))
  (bind _charactermovement (`self.CharacterMovement`))
  (:`Pressed`
    (set `CharacterMovementComponent.MaxWalkSpeed` (`self.RunSpeed`) _charactermovement)
    (set `self.FootstepInterval` 0.35)
    (`self.ResetSpeed` :!label _label))
  (:`Released`
    (set `CharacterMovementComponent.MaxWalkSpeed` (`self.WalkSpeed`) _charactermovement)
    (set `self.FootstepInterval` 0.55)
    (goto _label)))

(event `self.ReceiveBeginPlay`
  (set `CharacterMovementComponent.MaxWalkSpeed` (`self.WalkSpeed`) (`self.CharacterMovement`))
  (bind _returnvalue (`|CreateWidget` "/Game/ProjectHotelHorror/UserInterface/Widgets/WBP_Reticle_01.WBP_Reticle_01_C" (`GameplayStatics.GetPlayerController` 0)))
  (`UserWidget.AddToViewport` _returnvalue 0))

(event `InputAxis|MoveRight`
  (params (AxisValue :type "Float (single-precision)"))
  (bind (_returnvalue_roll _returnvalue_pitch _returnvalue_yaw) (`KismetMathLibrary.BreakRotator` (`self.GetControlRotation`)))
  (bind (_returnvalue_x _returnvalue_y _returnvalue_z) (`KismetMathLibrary.BreakVector` (`self.GetVelocity`)))
  (`self.AddMovementInput` (`KismetMathLibrary.GetRightVector` (`KismetMathLibrary.MakeRotator` 0.0 0.0 _returnvalue_yaw)) AxisValue)
  ;[1 1 1] Check if Player is moving for Footstep SFX...
  (if (and (or (> _returnvalue_x 2.0) (< _returnvalue_x -2.0) (> _returnvalue_y 2.0) (< _returnvalue_y -2.0)) (== _returnvalue_z 0.0)) :!label _label_2
    ;[1 1 1] Footstep SFX
    (`/Engine/EditorBlueprintResources/StandardMacros.DoOnce` false :!label _label_3
      (:`Completed`
        (bind _returnvalue (`KismetSystemLibrary.K2_SetTimerDelegate` (delegate `CheckPhysicsMaterial`) (`self.FootstepInterval`) true))
        (`self.CheckPhysicsMaterial`)))
    (else
      (`KismetSystemLibrary.K2_ClearAndInvalidateTimerHandle` _returnvalue :!label _label_4)
      (goto _label_3 :!via `Reset`))))

(event `ResetSpeed`
  ;[1 1 1] Footstep SFX
  (goto _label_4))

(event `InputAxis|MoveForward`
  (params (AxisValue :type "Float (single-precision)"))
  (bind (_returnvalue_roll _returnvalue_pitch _returnvalue_yaw) (`KismetMathLibrary.BreakRotator` (`self.GetControlRotation`)))
  (`self.AddMovementInput` (`KismetMathLibrary.GetForwardVector` (`KismetMathLibrary.MakeRotator` 0.0 0.0 _returnvalue_yaw)) AxisValue)
  (goto _label_2))

(event `CheckPhysicsMaterial`
  (bind _returnvalue (`self.K2_GetActorLocation`))
  ;[1 1 1] Footstep SFX
  (bind (_outhit _returnvalue_2) (`KismetSystemLibrary.LineTraceSingle` _returnvalue (- _returnvalue (0.0 0.0 150.0)) "TraceTypeQuery1"))
  (if _returnvalue_2
    (switch `EPhysicalSurface` (`GameplayStatics.GetSurfaceType` _outhit)
      (:`SurfaceType1`
        (`GameplayStatics.PlaySoundAtLocation` "/Game/ProjectHotelHorror/Characters/Common/Audio/Footsteps/A_Footsteps_Carpet_01.A_Footsteps_Carpet_01" _returnvalue (struct) 1.0 1.0 0.0 null null null))
      (:`SurfaceType11`
        (`GameplayStatics.PlaySoundAtLocation` "/Game/ProjectHotelHorror/Characters/Common/Audio/Footsteps/A_Footsteps_Wood_01.A_Footsteps_Wood_01" _returnvalue (struct) 1.0 1.0 0.0 null null null)))))

(event `self.ReceiveTick`
  (params (DeltaSeconds :type "Float (single-precision)"))
  (`self.HeadBob`)
  (if (`self.bInteracting`)
    (message `/Game/ProjectHotelHorror/Core/BPI_Interact.InteractMouse` (`self.InteractActor`) (* (`self.GetInputAxisValue`) -1.0) (`self.GetInputAxisValue`) (0.0 0.0 0.0))
    (`self.AddControllerYawInput` (* (`self.GetInputAxisValue`) 0.1))
    (`self.AddControllerPitchInput` (* (`self.GetInputAxisValue`) 0.1))
    (else
      (`self.AddControllerYawInput` (`self.GetInputAxisValue`))
      (`self.AddControllerPitchInput` (`self.GetInputAxisValue`)))))

(event `HeadBob`
  (bind _returnvalue (`GameplayStatics.GetPlayerController` 0))
  (bind _returnvalue_2 (`KismetMathLibrary.VSize` (`self.GetVelocity`)))
  (if (and (> _returnvalue_2 0.0) (`self.CanJump`))
    (if (< _returnvalue_2 300.0)
      (`PlayerController.ClientStartCameraShake` :`self` _returnvalue :`Shake` "/Game/ProjectHotelHorror/Core/BP_HeadBob_Walk_01.BP_HeadBob_Walk_01_C")
      (else
        (`PlayerController.ClientStartCameraShake` :`self` _returnvalue :`Shake` "/Game/ProjectHotelHorror/Core/BP_HeadBob_Run_01.BP_HeadBob_Run_01_C")))))

(event `InputAction|InteractInput`
  (params (Key :type "Key Structure"))
  (bind _returnvalue (`SceneComponent.K2_GetComponentLocation` (`self.Camera`)))
  ;[1 1 1] RE Style Open Doors
  (:`Pressed`
    (bind _outhit (`KismetSystemLibrary.LineTraceSingleForObjects` :`Start` _returnvalue :`End` (+ _returnvalue (* (`KismetMathLibrary.GetForwardVector` (`self.GetControlRotation`)) 200.0)) :`ObjectTypes` (`|MakeArray` "ObjectTypeQuery2" :!type "EObjectTypeQuery Enum") :`DrawDebugType` "Persistent"))
    (bind _asbp_hotel_room_door_single_01 (cast `/Game/Developers/ColeT/Placeables/Doors/BP_Hotel_Room_Door_Single_01` (`.HitActor` (`GameplayStatics.BreakHitResult` _outhit))))
    (`/Game/Developers/ColeT/Placeables/Doors/BP_Hotel_Room_Door_Single_01.InteractingWithDoor` _asbp_hotel_room_door_single_01 self)))

(event `/Game/ProjectHotelHorror/Core/BPI_Interact.InteractSuccesful`
  (params (Door :type "Actor Object Reference"))
  ;[1 1 1] AMNESIA STYLED DRAG DOORS CODE
  (set `self.InteractActor` Door)
  (set `self.bInteracting` true))

(fn `UserConstructionScript`)