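; BP_LevelManager runs an accelerated in-game clock for the level.
; A looping timer started on BeginPlay increments a seconds counter about 16.67 times per real second and converts it into a Timespan.
; An AdvanceTime event skips the counter ahead six hours.
; Event Tick prints the days, hours, minutes and seconds on screen every frame.
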(event `self.ReceiveBeginPlay`
  (`KismetSystemLibrary.K2_SetTimer` null "IncreaseTime" (/ 1.0 16.6667) true))

(event `IncreaseTime`
  (bind _result (`/Engine/EditorBlueprintResources/StandardMacros.IncrementInt` (`self.Tick`))
    (:`  `
      (set `self.Time` (`KismetMathLibrary.MakeTimespan` 0 0 0 _result)))))

(event `self.ReceiveTick`
  (params (DeltaSeconds :type "Float (single-precision)"))
  (bind (_days _hours _minutes _seconds) (`KismetMathLibrary.BreakTimespan` (`self.Time`)))
  (`KismetSystemLibrary.PrintString` (`KismetStringLibrary.Concat_StrStr` (`KismetStringLibrary.Conv_IntToString` _days) ":" (`KismetStringLibrary.Conv_IntToString` _hours) ":" (`KismetStringLibrary.Conv_IntToString` _minutes) ":" (`KismetStringLibrary.Conv_IntToString` _seconds)) true true (struct :`G` 0.66 :`B` 1.0 :`A` 1.0) (`GameplayStatics.GetWorldDeltaSeconds`)))

(event `AdvanceTime`
  (set `self.Tick` (+ (`self.Tick`) 21600)))

(fn `UserConstructionScript`)